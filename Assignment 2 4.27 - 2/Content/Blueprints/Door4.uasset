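; Door actor that slides open for a BP_Key whose material matches the door's own.
; Box overlap casts the other actor to BP_Key and compares slot 0 materials of the key's and door's Cube components as strings.
; On a match, a timeline drives DoorUp's relative Z.
; Ending any overlap with the box reverses the timeline, with no key check.
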(event OnComponentBeginOverlap(Box)
  (params (OverlappedComponent :type Primitive%20Component%20Object%20Reference) (OtherActor :type Actor%20Object%20Reference) (OtherComp :type Primitive%20Component%20Object%20Reference) (OtherBodyIndex :type Integer) (bFromSweep :type Boolean) (SweepResult :type Hit%20Result%20Structure%20%28by%20ref%29))
  ;[1 1 1 1 30] Interacting with the Key(cube) and the Door Open
  ;;[1 1 1] Basically on the Box Collision casting with BP_Key and set a condition if it is the material is True or Equal the Door will open and i add a cube component component to my door.
  (bind _asbp_key (Utilities|Casting|CastToBP_Key OtherActor))
  (bind _output_get (Variables|Default|SetcubeIdentifier _asbp_key))
  (if (Utilities|Enum|Equal(Enum) (Utilities|String|ToString(Object) (Rendering|Material|GetMaterial (Variables|/Game/Blueprints/BP_Key.BP_Key_C|GetCube _output_get) 0)) (Utilities|String|ToString(Object) (Rendering|Material|GetMaterial (Variables|Default|GetCube) 0)))
    (bind _newtrack_0 (Timeline|Timeline_0 Play)
      (:Update
        (Transformation|SetRelativeLocation (Variables|Default|GetDoorUp) (Math|Vector|MakeVector 0.0 0.0 _newtrack_0) false false)))))

(event OnComponentEndOverlap(Box)
  (params (OverlappedComponent :type Primitive%20Component%20Object%20Reference) (OtherActor :type Actor%20Object%20Reference) (OtherComp :type Primitive%20Component%20Object%20Reference) (OtherBodyIndex :type Integer))
  ;[1 1 1 1 30] Interacting with the Key(cube) and the Door Open
  ;;[1 1 1] Reverse, the door will close
  ;;[1 1 1] Basically on the Box Collision casting with BP_Key and set a condition if it is the material is True or Equal the Door will open and i add a cube component component to my door.
  (bind _newtrack_0 (Timeline|Timeline_0 Reverse)
    (:Update
      (Transformation|SetRelativeLocation (Variables|Default|GetDoorUp) (Math|Vector|MakeVector 0.0 0.0 _newtrack_0) false false))))

(event EventBeginPlay)

(event Collision|EventActorBeginOverlap
  (params (OtherActor :type Actor%20Object%20Reference)))

(event EventTick
  (params (DeltaSeconds :type Float%20%28single-precision%29)))

(fn ConstructionScript)