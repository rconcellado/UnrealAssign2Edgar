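; BP_PaintBucket is an interactable that repaints a BP_Key cube, changing which door name the key carries.
; Box overlap events store the key, toggle whether painting is allowed, and print the key's SegmentName.
; While enabled, pressing C cycles through three door names with matching gold, steel and rust materials.
; The cycle counter lives on the bucket, so it is independent of each key's current state.
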(event OnComponentBeginOverlap(Box)
  (params (OverlappedComponent :type Primitive%20Component%20Object%20Reference) (OtherActor :type Actor%20Object%20Reference) (OtherComp :type Primitive%20Component%20Object%20Reference) (OtherBodyIndex :type Integer) (bFromSweep :type Boolean) (SweepResult :type Hit%20Result%20Structure%20%28by%20ref%29))
  ;[1 1 1] Interacting with the BP_Key(Cube)
  (bind _output_get (Variables|Default|SetobjectiveIdentifier OtherActor))
  (bind _asbp_key (Utilities|Casting|CastToBP_Key _output_get))
  (Variables|Default|SetcubeIdentifier _asbp_key)
  (Variables|Default|SettransformColor true)
  (Development|PrintString (Variables|/Game/Blueprints/BP_Key.BP_Key_C|GetsegmentName (Variables|Default|GetcubeIdentifier))))

(event OnComponentEndOverlap(Box)
  (params (OverlappedComponent :type Primitive%20Component%20Object%20Reference) (OtherActor :type Actor%20Object%20Reference) (OtherComp :type Primitive%20Component%20Object%20Reference) (OtherBodyIndex :type Integer))
  ;[1 1 1] Interacting with the BP_Key(Cube)
  (bind _output_get (Variables|Default|SetobjectiveIdentifier OtherActor))
  (bind _asbp_key (Utilities|Casting|CastToBP_Key _output_get))
  (Variables|Default|SetcubeIdentifier _asbp_key)
  (Variables|Default|SettransformColor false)
  (Development|PrintString (Variables|/Game/Blueprints/BP_Key.BP_Key_C|GetsegmentName (Variables|Default|GetcubeIdentifier))))

(event Input|KeyboardEvents|C
  (params (Key :type Key%20Structure :default "None"))
  (bind _cubeidentifier (Variables|Default|GetcubeIdentifier))
  (bind _cubeidentifier_2 (Variables|Default|GetcubeIdentifier))
  (bind _cube (Variables|/Game/Blueprints/BP_Key.BP_Key_C|GetCube _cubeidentifier_2))
  ;[1 1 1] Key Press 'C' to Change the Material of the Cube(Key)
  (:Pressed
    (if (Variables|Default|GettransformColor)
      (switch int (Variables|Default|GettallyCounter)
        (:0
          (Variables|/Game/Blueprints/BP_Key.BP_Key_C|SetsegmentName _cubeidentifier "Door 1")
          (Rendering|Material|SetMaterial _cube 0 "/Game/StarterContent/Materials/M_Metal_Gold.M_Metal_Gold")
          (Variables|Default|SettallyCounter 1))
        (:1
          (Variables|/Game/Blueprints/BP_Key.BP_Key_C|SetsegmentName _cubeidentifier "Door 2")
          (Rendering|Material|SetMaterial _cube 0 "/Game/StarterContent/Materials/M_Metal_Steel.M_Metal_Steel")
          (Variables|Default|SettallyCounter 2))
        (:2
          (Variables|/Game/Blueprints/BP_Key.BP_Key_C|SetsegmentName _cubeidentifier "Door 3")
          (Rendering|Material|SetMaterial _cube 0 "/Game/StarterContent/Materials/M_Metal_Rust.M_Metal_Rust")
          (Variables|Default|SettallyCounter 0))))))

(fn ConstructionScript)